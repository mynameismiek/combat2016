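; Cannon weapon component that fires projectiles from the Muzzle socket of a supplied mesh.
; FireWeapon is gated by a CanFire flag and requires a Pawn owner, which becomes the projectile's instigator.
; Each shot spawns the projectile, muzzle particles and firing sound at the socket, plus a world camera shake oriented toward the muzzle.
; A Delay of FiringRate then re-enables firing, acting as a cooldown.
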(event EventBeginPlay)

(event EventTick
  (params (DeltaSeconds :type Float%20%28single-precision%29)))

(event EventFireWeapon
  (params (From%20Mesh :type Mesh%20Component%20Object%20Reference))
  (bind _returnvalue (Transformation|GetSocketTransform From%20Mesh "Muzzle" "RTS_World"))
  (bind _returnvalue_2 (Components|GetOwner))
  (bind (_location _rotation) (Math|Transform|BreakTransform _returnvalue))
  (if (Variables|Default|GetCan%20Fire)
    (Variables|Default|SetCan%20Fire false)
    (bind _aspawn (Utilities|Casting|CastToPawn _returnvalue_2))
    (Effects|SpawnEmitteratLocation (Variables|Default|GetFiringParticles) _location _rotation)
    (Game|SpawnActorfromClass "/Game/Blueprints/CannonProjectile.CannonProjectile_C" _returnvalue "AlwaysSpawn" _returnvalue_2 _aspawn)
    (Audio|PlaySoundatLocation (Variables|Default|GetFiring%20Sound%20Cue) _location)
    (Camera|PlayWorldCameraShake "/Game/Blueprints/Cam_CannonFiring_Shake.Cam_CannonFiring_Shake_C" _location 0.0 8e+03 1.0 true)
    (Utilities|FlowControl|Delay (Variables|Default|GetFiring%20Rate))
    (Variables|Default|SetCan%20Fire true)))