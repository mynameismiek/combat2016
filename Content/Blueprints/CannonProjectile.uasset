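; CannonProjectile is a projectile actor that damages whatever actor it hits.
; On overlap with any actor other than its Instigator, it plays an explosion sound at its location, applies its Damage value crediting the Instigator's controller, then destroys itself.
; All logic lives in that one overlap event; the graphs contain no movement, Tick or construction logic.
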(event EventBeginPlay)

(event EventActorBeginOverlap
  (params (OtherActor :type Actor%20Object%20Reference))
  (bind _instigator (Variables|Actor|GetInstigator))
  (if (!= OtherActor _instigator)
    (Audio|PlaySoundatLocation (Variables|Default|GetExplosionSoundCue) (Transformation|GetActorLocation))
    (Game|Damage|ApplyDamage OtherActor (Variables|Default|GetDamage) (Pawn|GetController _instigator) self)
    (Actor|DestroyActor)))

(event EventTick
  (params (DeltaSeconds :type Float%20%28single-precision%29)))

(fn ConstructionScript)