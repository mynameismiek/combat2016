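; CombatPlayerController is a player controller for driving wheeled vehicles under a level-placed combat camera.
; On BeginPlay it finds the first CombatCamera actor in the world and instantly switches the view target to it.
; Forward and right input axes cast the controlled pawn to WheeledVehicle and feed its movement component's throttle and steering.
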(event EventBeginPlay
  (bind _outactors (Actor|GetAllActorsOfClass "/Game/Blueprints/CombatCamera.CombatCamera_C"))
  (Game|Player|SetViewTargetwithBlend (Utilities|Array|Get(acopy) _outactors) 0.0 "VTBlend_Linear" 0.0 false))

(event EventTick
  (params (DeltaSeconds :type Float%20%28single-precision%29)))

(event Input|AxisEvents|InputAxisMovementForward
  (params (AxisValue :type Float%20%28single-precision%29))
  (bind _aswheeled_vehicle (Utilities|Casting|CastToWheeledVehicle (Pawn|GetControlledPawn)))
  (Class|WheeledVehicleMovementComponent|SetThrottleInput (Variables|/Script/Engine.WheeledVehicle|GetVehicleMovement _aswheeled_vehicle) AxisValue))

(event Input|AxisEvents|InputAxisMoveRight
  (params (AxisValue :type Float%20%28single-precision%29))
  (bind _aswheeled_vehicle (Utilities|Casting|CastToWheeledVehicle (Pawn|GetControlledPawn)))
  (Class|WheeledVehicleMovementComponent|SetSteeringInput (Variables|/Script/Engine.WheeledVehicle|GetVehicleMovement _aswheeled_vehicle) AxisValue))

(fn ConstructionScript)