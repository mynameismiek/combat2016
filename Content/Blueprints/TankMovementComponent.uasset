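; Tank movement component that drives and turns its owning Pawn and gives it an engine sound.
; On BeginPlay it caches the owner as a Pawn and spawns the engine cue attached to its root, with attenuation.
; OnForward and OnRight events take axis values and apply local X offset and yaw rotation, scaled by maximum speeds and delta seconds.
; It moves the actor transform directly, with no acceleration or physics forces.
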(event Custom|On%20Forward
  (params (Axis%20Value :type Float%20%28single-precision%29))
  (CallFunction|ForwardHandler Axis%20Value))

(event Custom|On%20Right
  (params (Axis%20Value :type Float%20%28single-precision%29))
  (CallFunction|RightHandler Axis%20Value))

(event EventBeginPlay
  (bind _aspawn (Utilities|Casting|CastToPawn (Components|GetOwner))
    (:then
      (Variables|Default|SetOwning%20Pawn _aspawn))
    (:CastFailed
      _))
  (CallFunction|SetupEngineSound))

(event EventTick
  (params (DeltaSeconds :type Float%20%28single-precision%29)))

(fn RightHandler
  (params (A :type Float%20%28single-precision%29))
  (Transformation|AddActorLocalRotation (Variables|Default|GetOwning%20Pawn) (Math|Rotator|MakeRotator 0.0 0.0 (* (Utilities|Time|GetWorldDeltaSeconds) (* A (Variables|Default|GetMaximumRotationSpeed)))) false false)
  (return))

(fn ForwardHandler
  (params (A :type Float%20%28single-precision%29))
  (Transformation|AddActorLocalOffset (Variables|Default|GetOwning%20Pawn) (Math|Vector|MakeVector (* (Utilities|Time|GetWorldDeltaSeconds) (* A (Variables|Default|GetMaximumForwardSpeed))) 0.0 0.0) false false)
  (return))

(fn SetupEngineSound
  (Audio|SpawnSoundAttached (Variables|Default|GetEngine%20Sound%20Cue) (VehicleSound|GetRootComponent (Variables|Default|GetOwning%20Pawn)) "None" "0, 0, 0" "0, 0, 0" "SnapToTargetIncludingScale" true 1.0 1.0 0.0 (Variables|Default|GetEngine%20Attenuation))
  (return))