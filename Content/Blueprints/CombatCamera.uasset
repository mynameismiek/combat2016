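; Shared combat camera actor that follows the average position of all players and zooms to fit their spread.
; On the authority, each tick averages player pawn locations at zero height, then sets zoom from twice the farthest pawn distance, clamped to limits.
; RepNotify handlers on target location and zoom move the actor and set camera arm length.
; A debug string displays the current zoom.
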(event EventBeginPlay
  (Networking|SwitchHasAuthority
    (:Authority
      (bind _output_get (Variables|Default|SetCurrentLocation (Transformation|GetActorLocation)))
      (Variables|Default|SetTargetLocation _output_get))))

(event EventActorBeginOverlap
  (params (OtherActor :type Actor%20Object%20Reference)))

(event EventTick
  (params (DeltaSeconds :type Float%20%28single-precision%29))
  (bind _returnvalue (Game|GetGameState))
  (bind _playerarray (Variables|/Script/Engine.GameState|GetPlayerArray _returnvalue))
  (Networking|SwitchHasAuthority
    (:Authority
      (Utilities|FlowControl|Sequence
        (:then_0
          ;[1 1 1] Figure out where the Camera SHOULD be located based on player locations
          (Variables|Default|SetPlayerPawnLocations "0, 0, 0")
          (for (_ _array_index) _playerarray
            (Variables|Default|SetPlayerPawnLocations (+ (Variables|Default|GetPlayerPawnLocations) (Transformation|GetActorLocation (Pawn|GetControlledPawn (Game|GetPlayerController _array_index))))))
          (Variables|Default|SetTargetLocation (Math|Vector|MakeVector (.X (Math|Vector|BreakVector (/ (Variables|Default|GetPlayerPawnLocations) (Utilities|Array|Length _playerarray)))) (.Y (Math|Vector|BreakVector (/ (Variables|Default|GetPlayerPawnLocations) (Utilities|Array|Length _playerarray)))) 0.0)))
        (:then_1
          (CallFunction|CalculateZoom))
        (:then_2
          (Rendering|Debug|DrawDebugString "0, 0, 0" (Utilities|String|Append "Zoom: " (Utilities|String|ToString(Float) (Variables|Default|GetCurrentZoom))) 0 "(R=1.000000,G=1.000000,B=1.000000,A=1.000000)"))))))

(fn ConstructionScript)

(fn OnRepTargetLocation
  (Transformation|SetActorLocation (Variables|Default|GetTargetLocation) false false))

(fn OnRepCurrentZoom
  (Variables|/Script/Engine.SpringArmComponent|SetTargetArmLength (Variables|Default|GetCameraArm) (Variables|Default|GetCurrentZoom)))

(fn CalculateZoom
  (for (_ _array_index) (Variables|/Script/Engine.GameState|GetPlayerArray (Game|GetGameState))
    (if (> (Math|Vector|VectorLength (- (Variables|Default|GetTargetLocation) (Transformation|GetActorLocation (Pawn|GetControlledPawn (Game|GetPlayerController _array_index))))) (LocalVariables|GetLongestVector))
      (LocalVariables|SetLongestVector (Math|Vector|VectorLength (- (Variables|Default|GetTargetLocation) (Transformation|GetActorLocation (Pawn|GetControlledPawn (Game|GetPlayerController _array_index))))))))
  ;[1 1 1] Figure out the Camera Zoom based on player locations
  (Variables|Default|SetCurrentZoom (Math|Float|Clamp(Float) (* (LocalVariables|GetLongestVector) 2.0) (Variables|Default|GetMinZoom) (Variables|Default|GetMaxZoom)))
  (return))